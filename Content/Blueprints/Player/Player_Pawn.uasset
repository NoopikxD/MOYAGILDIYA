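; Player pawn for point-and-click movement and interaction with world objects through interfaces.
; Each tick it traces under the cursor to place a cursor marker and drive hover highlights, and ends interactions that fall out of range.
; Clicking interacts with items in range, otherwise starts controller movement, then interacts once the clicked item is within range.
; Other inputs highlight all items via GameState, open context menus and toggle the inventory.
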(event `Initialize`
  (`|ExecutionSequence`
    (:`then_0`
      (bind _asmy_game_state (cast `/Game/Blueprints/MyGameState` (`GameplayStatics.GetGameState`)))
      (set `self.GameStateRef` _asmy_game_state))
    (:`then_1`
      (bind _asplayer_controller (cast `/Game/Blueprints/Player/Player_Controller` (`self.GetController`)))
      (set `self.ControllerRef` _asplayer_controller))))

(event `self.ReceiveBeginPlay`
  (`|ExecutionSequence`
    (:`then_0`
      (`self.Initialize`))))

(event `TargetReached`
  (params (Target :type "Actor Object Reference"))
  (`self.OnTargetReached` Target)
  (`/Engine/EditorBlueprintResources/StandardMacros.IsValid` (`self.CurrentInteractionObject`)
    (:`Is Not Valid`
      (if (`KismetSystemLibrary.DoesImplementInterface` Target "/Game/Blueprints/Items/IInteractibleItems.IInteractibleItems_C")
        (bind _output_get (set `self.CurrentInteractionObject` Target))
        (message `/Game/Blueprints/Items/IInteractibleItems.StartInteraction` _output_get self)))))

(event `self.ReceiveTick`
  (params (DeltaSeconds :type "Float (single-precision)"))
  (`|ExecutionSequence`
    (:`then_0`
      (`self.TraceCursorLocation`))
    (:`then_1`
      (`self.TraceDistanceToCurrentInteractionObj`))
    (:`then_2`
      (`self.TraceDistanceToLastHitActor`))))

(event `MouseOverActor`
  (params (Actor :type "Actor Object Reference"))
  (if (not (`self.isHigliteMode`))
    (`/Engine/EditorBlueprintResources/StandardMacros.IsValid` Actor
      (:`Is Valid`
        (if (`KismetSystemLibrary.DoesImplementInterface` Actor "/Game/Blueprints/Items/IInteractibleItems.IInteractibleItems_C")
          (message `/Game/Blueprints/Items/IInteractibleItems.OnStartHighlite` Actor self))))))

(event `MouseLeaveActor`
  (params (Actor :type "Actor Object Reference"))
  (if (not (`self.isHigliteMode`))
    (`/Engine/EditorBlueprintResources/StandardMacros.IsValid` Actor
      (:`Is Valid`
        (if (`KismetSystemLibrary.DoesImplementInterface` Actor "/Game/Blueprints/Items/IInteractibleItems.IInteractibleItems_C")
          (message `/Game/Blueprints/Items/IInteractibleItems.OnEndHighlite` Actor self))))))

(event `InputAction|HighliteItems`
  (params (Key :type "Key Structure"))
  (:`Pressed`
    (set `self.isHigliteMode` true)
    (message `/Game/Blueprints/Items/IInteractibleItems.OnEndHighlite` (`self.ActorUnderMouse`) self)
    (`/Game/Blueprints/MyGameState.StartHighliteInteractibleItems` (`self.GameStateRef`)))
  (:`Released`
    (set `self.isHigliteMode` false)
    (message `/Game/Blueprints/Items/IInteractibleItems.OnStartHighlite` (`self.ActorUnderMouse`) self)
    (`/Game/Blueprints/MyGameState.EndHighliteInteractibleItems` (`self.GameStateRef`))))

(event `InputAction|Move/Use`
  (params (Key :type "Key Structure"))
  (bind _currentinteractionobject (`self.CurrentInteractionObject`))
  (bind _controllerref (`self.ControllerRef`))
  (bind _actorundermouse (`self.ActorUnderMouse`))
  (:`Pressed`
    (`/Engine/EditorBlueprintResources/StandardMacros.IsValid` _actorundermouse
      (:`Is Valid`
        (set `self.MouseLastHitActor` _actorundermouse)
        (if (`KismetSystemLibrary.DoesImplementInterface` _actorundermouse "/Game/Blueprints/Items/IInteractibleItems.IInteractibleItems_C")
          (if (<= (`self.GetHorizontalDistanceTo` self _actorundermouse) (`self.InteractionDistance`))
            (if (!= _actorundermouse (`self.CurrentInteractionObject`))
              (`|ExecutionSequence`
                (:`then_0`
                  (`/Engine/EditorBlueprintResources/StandardMacros.IsValid` _currentinteractionobject
                    (:`Is Valid`
                      (message `/Game/Blueprints/Items/IInteractibleItems.EndInteraction` _currentinteractionobject self))))
                (:`then_1`
                  (bind _output_get (set `self.CurrentInteractionObject` (`self.ActorUnderMouse`)))
                  (message `/Game/Blueprints/Items/IInteractibleItems.StartInteraction` _output_get self))))
            (else
              (`/Game/Blueprints/Player/Player_Controller.StartMovementMouseHOld` _controllerref :!label _label)))
          (else
            (goto _label))))
      (:`Is Not Valid`
        (goto _label))))
  (:`Released`
    (`/Game/Blueprints/Player/Player_Controller.EndMovementMouseHold` _controllerref)
    (`self.DeactivateContextMenu`)))

(event `InputAction|ContextMEnu`
  (params (Key :type "Key Structure"))
  (bind _actorundermouse (`self.ActorUnderMouse`))
  (bind _actorundermouse_2 (`self.ActorUnderMouse`))
  (:`Pressed`
    (`self.DeactivateContextMenu`)
    (`/Engine/EditorBlueprintResources/StandardMacros.IsValid` _actorundermouse_2
      (:`Is Valid`
        (if (`KismetSystemLibrary.DoesImplementInterface` _actorundermouse_2 "/Game/Blueprints/UI/ContextMenu/IContextInteractible.IContextInteractible_C")
          (message `/Game/Blueprints/UI/ContextMenu/IContextInteractible.ContextActivate` _actorundermouse true)
          (set `self.CurrentContextInteractionObject` _actorundermouse))))))

(event `InputAction|Inventory`
  (params (Key :type "Key Structure"))
  (bind _inventorycomponent (`self.InventoryComponent`))
  (:`Pressed`
    (`/Engine/EditorBlueprintResources/StandardMacros.FlipFlop`
      (:`A`
        (`/Game/Blueprints/Inventory/InventoryCOmponent.OpenInventory` _inventorycomponent))
      (:`B`
        (`/Game/Blueprints/Inventory/InventoryCOmponent.CloseInventory` _inventorycomponent)))))

(fn `DeactivateContextMenu`
  (bind _currentcontextinteractionobject (`self.CurrentContextInteractionObject`))
  (`/Engine/EditorBlueprintResources/StandardMacros.IsValid` _currentcontextinteractionobject
    (:`Is Valid`
      (message `/Game/Blueprints/UI/ContextMenu/IContextInteractible.ContextDeactivate` _currentcontextinteractionobject)
      (set `self.CurrentContextInteractionObject` null))))

(fn `UserConstructionScript`)