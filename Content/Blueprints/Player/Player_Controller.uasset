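; Player controller for click-and-hold movement of the Player_Pawn, with interaction on arrival.
; While held, a gated Tick macro traces under the cursor and either calls SimpleMoveToLocation or, within InteractionDistance, reports interactible actors to the pawn.
; A second gate re-checks a stored MoveLocation each frame, firing CallOnTargetReached once within range.
; Tick also snaps any actor passed to AttachToMouse to the WorldStatic point under the cursor.
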(event `self.ReceiveTick`
  (params (DeltaSeconds :type "Float (single-precision)"))
  (bind _attachedactor (`self.attachedActor`))
  ;[1 1 1] Click and go there
  (`|ExecutionSequence`
    (:`then_0`
      (`self.MoveToLocationMouseHold` :!label _label))
    (:`then_1`
      (`/Engine/EditorBlueprintResources/StandardMacros.Gate` true :!label _label_2
        (:`Exit`
          (`self.MoveToLocation` (`self.MoveLocation`)))))
    (:`then_2`
      (`/Engine/EditorBlueprintResources/StandardMacros.IsValid` _attachedactor
        (:`Is Valid`
          (`self.K2_SetActorLocation` _attachedactor (`.Location` (`GameplayStatics.BreakHitResult` (`self.GetHitResultUnderCursorForObjects` (`|MakeArray` "ObjectTypeQuery1" :!type "EObjectTypeQuery Enum")))) false false))))))

(event `StartMovementMouseHOld`
  ;[1 1 1] Click and go there
  (goto _label :!via `Open`))

(event `EndMovementMouseHold`
  ;[1 1 1] Click and go there
  (goto _label :!via `Close`))

(event `StartMoveToLocation`
  ;[1 1 1] Click and go there
  (goto _label_2 :!via `Open`))

(event `EndMoveToLocation`
  ;[1 1 1] Click and go there
  (goto _label_2 :!via `Close`))

(event `self.ReceiveBeginPlay`
  (bind _asplayer_pawn (cast `/Game/Blueprints/Player/Player_Pawn` (`GameplayStatics.GetPlayerPawn` 0)))
  (set `self.PlayerRef` _asplayer_pawn))

(event `MoveToLocation`
  (params (Location :type "Vector Structure"))
  (set `self.MoveLocation` Location)
  (if (>= (`KismetMathLibrary.VSize` (* (- Location (`self.K2_GetActorLocation` (`self.K2_GetPawn`))) (1.0 1.0 0.0))) (`/Game/Blueprints/Player/Player_Pawn.InteractionDistance` (`self.PlayerRef`)))
    (`self.StartMoveToLocation`)
    (else
      (`/Game/Blueprints/Player/Player_Pawn.OnTargetReached` (`self.PlayerRef`) null)
      (`self.EndMoveToLocation`))))

(fn `AttachToMouse`
  (params (Actor :type "Actor Object Reference"))
  (set `self.attachedActor` Actor))

(fn `MoveToHitLocation`
  (params (Hit :type "HitResult Structure"))
  (bind (_bblockinghit _binitialoverlap _time _distance _location _impactpoint _normal _impactnormal _physmat _hitactor) (`GameplayStatics.BreakHitResult` Hit))
  (if (>= (`KismetMathLibrary.VSize` (* (- (`self.K2_GetActorLocation` (`self.K2_GetPawn`)) _location) (1.0 1.0 0.0))) (`/Game/Blueprints/Player/Player_Pawn.InteractionDistance` (`self.PlayerRef`)))
    (`AIBlueprintHelperLibrary.SimpleMoveToLocation` self _location)
    (elif (`KismetSystemLibrary.DoesImplementInterface` _hitactor "/Game/Blueprints/Items/IInteractibleItems.IInteractibleItems_C")
      (`/Game/Blueprints/Player/Player_Pawn.TargetReached` (`self.PlayerRef`) _hitactor))))

(fn `UserConstructionScript`)