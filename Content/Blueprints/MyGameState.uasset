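; Game state Blueprint that tracks the level's interactible items and toggles their highlight.
; On BeginPlay it caches every actor implementing the InteractibleItems interface, and the getter returns that cache unless it is empty, in which case it searches again.
; Start and end highlight functions loop over the cached array and send each actor the matching interface message.
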(event `self.ReceiveBeginPlay`
  (`parent.ReceiveBeginPlay`)
  (`|ExecutionSequence`
    (:`then_0`
      (bind _items (`self.GetAllInteractibleItems`))
      (set `self.InteractibleItems` _items))))

(event `self.ReceiveTick`
  (params (DeltaSeconds :type "Float (single-precision)")))

(fn `EndHighliteInteractibleItems`
  (for _array_element (`self.InteractibleItems`)
    (message `/Game/Blueprints/Items/IInteractibleItems.OnEndHighlite` _array_element null)))

(fn `GetAllInteractibleItems`
  (returns (Items :type "Array of Actor Object Reference"))
  (if (> (`KismetArrayLibrary.Array_Length` (`self.InteractibleItems`)) 0)
    (return (`self.InteractibleItems`))
    (else
      (bind _outactors (`GameplayStatics.GetAllActorsWithInterface` "/Game/Blueprints/Items/IInteractibleItems.IInteractibleItems_C"))
      (return _outactors))))

(fn `StartHighliteInteractibleItems`
  (for _array_element (`self.InteractibleItems`)
    (message `/Game/Blueprints/Items/IInteractibleItems.OnStartHighlite` _array_element null)))

(fn `UserConstructionScript`)