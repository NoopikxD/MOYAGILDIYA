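; Inventory component that stashes items in a fixed-size grid and drops them back into the world.
; It creates a UI_Inventory widget on BeginPlay, shows or hides it, and passes it item changes.
; A map pairs items with 2D slot positions, and a scanning cursor finds the next free slot.
; Removal traces under the mouse, dropping items within range or moving the player toward distant points, where the arrival handler only prints.
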(event `OpenInventory`
  (bind _widgetref (`self.WidgetRef`))
  (`UserWidget.AddToViewport` _widgetref 0)
  (`/Game/Blueprints/UI/Inventory/UI_Inventory.UpdateSlots` _widgetref (`self.StashedItems`)))

(event `CloseInventory`
  (`Widget.RemoveFromParent` (`self.WidgetRef`)))

(event `self.ReceiveBeginPlay`
  (bind _output_get (set `self.Rows` (/ (`self.SlotsNum`) (`self.Cols`))))
  (`KismetSystemLibrary.PrintString` (`KismetStringLibrary.Conv_IntToString` _output_get) true true (struct :`R` 1.0 :`G` 0.102836 :`A` 1.0))
  (bind _returnvalue (`|CreateWidget` "/Game/Blueprints/UI/Inventory/UI_Inventory.UI_Inventory_C" null (`self.Rows`) (`self.Cols`) self))
  (set `self.WidgetRef` _returnvalue))

(fn `DropItem`
  (params (Item :type "/Game/Blueprints/Inventory/InventoryItem Object Reference") (Location :type "Vector Structure"))
  (bind _stasheditems (`self.StashedItems`))
  (`BlueprintMapLibrary.Map_Remove` _stasheditems Item)
  (`|SpawnActorFromClass` (`/Game/Blueprints/Inventory/InventoryItem.ItemClass` Item) (`KismetMathLibrary.MakeTransform` Location) "Undefined" "OverrideRootScale" null null)
  (`/Game/Blueprints/UI/Inventory/UI_Inventory.UpdateStashedItems` (`self.WidgetRef`) _stasheditems))

(fn `OnTargetReached`
  (params (Target :type "Actor Object Reference"))
  (`KismetSystemLibrary.PrintString` "Hello" true true (struct :`R` 0.911847 :`B` 1.0 :`A` 1.0)))

(fn `RemoveFromInventory`
  (params (InventoryItem :type "/Game/Blueprints/Inventory/InventoryItem Object Reference") (MousePosition :type "Vector2D Structure"))
  (bind _returnvalue (`GameplayStatics.GetPlayerPawn` 0))
  (bind _returnvalue_2 (`GameplayStatics.GetPlayerController` 0))
  (bind (_worldlocation _worlddirection) (`PlayerController.DeprojectScreenPositionToWorld` _returnvalue_2 MousePosition_X MousePosition_Y))
  (bind _outhit (`KismetSystemLibrary.LineTraceSingleForObjects` _worldlocation (* _worlddirection (+ (`KismetMathLibrary.GetForwardVector` (`Controller.GetControlRotation` _returnvalue_2)) 12000.0)) (`|MakeArray` "ObjectTypeQuery1" :!type "EObjectTypeQuery Enum")))
  (bind (_bblockinghit _binitialoverlap _time _distance _location _impactpoint _normal _impactnormal _physmat _hitactor) (`GameplayStatics.BreakHitResult` _outhit))
  (if (<= (`KismetMathLibrary.VSize` (- (* _location (1.0 1.0 0.0)) (* (`Actor.K2_GetActorLocation` (`GameplayStatics.GetPlayerCharacter` 0)) (1.0 1.0 0.0)))) 300.0)
    (`/Engine/EditorBlueprintResources/StandardMacros.IsValid` _hitactor
      (:`Is Valid`
        (`self.DropItem` InventoryItem _location)))
    (else
      (bind _asplayer_pawn (cast `/Game/Blueprints/Player/Player_Pawn` _returnvalue))
      (add `/Game/Blueprints/Player/Player_Pawn.OnTargetReached` _asplayer_pawn (`|CreateDelegate` :!event `OnTargetReached`))
      (bind _asplayer_controller (cast `/Game/Blueprints/Player/Player_Controller` (`Pawn.GetController` _returnvalue)))
      (`/Game/Blueprints/Player/Player_Controller.MoveToLocation` _asplayer_controller _location))))

(fn `ResetFreeSlot`
  (returns (FirstFreeSlot :type "Vector2D Structure"))
  (bind _output_get (set `self.FirstFreeSlot` (0.0 0.0)))
  (bind _isavaliable (`self.CheckSlotAvaliability` _output_get)
    (:`Execute`
      (if (not _isavaliable)
        (`self.IncrementFreeSlot`
          (:`execute`
            _)
          (:`NoFreeSpace`
            (return (-1.0 -1.0)))))
      (return (`self.FirstFreeSlot`)))))

(fn `StashItem`
  (params (InventoryItem :type "/Game/Blueprints/Inventory/InventoryItem Object Reference"))
  (bind _stasheditems (`self.StashedItems`))
  (bind _widgetref (`self.WidgetRef`))
  (`BlueprintMapLibrary.Map_Add` _stasheditems InventoryItem (`self.FirstFreeSlot`))
  (`self.IncrementFreeSlot`
    (:`execute`
      (if (`Widget.IsInViewport` _widgetref)
        (`/Game/Blueprints/UI/Inventory/UI_Inventory.UpdateSlots` _widgetref _stasheditems)))))