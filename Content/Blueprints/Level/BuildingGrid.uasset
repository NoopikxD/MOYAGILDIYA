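; Building grid actor that fills a box area with BuildingGridCell child actors, built in the construction script.
; The box extent and cell width and height set the row and column counts, truncated to whole cells.
; A nested loop adds one child actor per cell, laid out from the positive X/Y corner, sizes its box to the cell and collects it in the Cells array.
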(fn `UserConstructionScript`
  (bind _cellwidth (`self.CellWidth`))
  (bind _cellheight (`self.CellHeight`))
  (bind (_boxextent_x _boxextent_y) (`KismetMathLibrary.BreakVector` (`self.BoxExtent`)))
  (bind (_boxextent_x_2 _boxextent_y_2) (`KismetMathLibrary.BreakVector` (`self.BoxExtent`)))
  (`KismetArrayLibrary.Array_Clear` (`self.Cells`))
  (`BoxComponent.SetBoxExtent` (`self.Box`) (`self.BoxExtent`) true)
  (`|ExecutionSequence`
    (:`then_0`
      (bind _output_get (set `self.CellsInRow` (`KismetMathLibrary.FTrunc` (/ (* _boxextent_x_2 2.0) (`self.CellWidth`)))))
      (bind _output_get_2 (set `self.CellsInCol` (`KismetMathLibrary.FTrunc` (/ (* _boxextent_y_2 2.0) (`self.CellHeight`)))))
      (set `self.CellNum` (* _output_get _output_get_2)))
    (:`then_1`
      (for _index (range (`self.CellsInRow`))
        (for _index_2 (range (`self.CellsInCol`))
          (bind _returnvalue (`AddComponent|NODE_AddChildActorComponent-0` :`RelativeTransform` (`KismetMathLibrary.MakeTransform` (`KismetMathLibrary.MakeVector` (- (- _boxextent_x (* _index _cellwidth)) (/ _cellwidth 2.0)) (- (- _boxextent_y (* _index_2 _cellheight)) (/ _cellheight 2.0))) (struct) (1.0 1.0 1.0))))
          (`ChildActorComponent.SetChildActorClass` _returnvalue "/Game/Blueprints/Level/BuildingGridCell.BuildingGridCell_C")
          (bind _asbuilding_grid_cell (cast `/Game/Blueprints/Level/BuildingGridCell` (`ChildActorComponent.ChildActor` _returnvalue)))
          (`BoxComponent.SetBoxExtent` (`/Game/Blueprints/Level/BuildingGridCell.Box` _asbuilding_grid_cell) (`KismetMathLibrary.MakeVector` (/ (`self.CellWidth`) 2.0) (/ (`self.CellHeight`) 2.0) 20.0) false)
          (`KismetArrayLibrary.Array_Add` (`self.Cells`) _asbuilding_grid_cell))))))