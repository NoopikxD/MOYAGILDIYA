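; Base actor for world items that a player can pick up and stash in an inventory.
; On interaction it checks the player's InventoryComponent for space, stores a new InventoryItem holding its name, weight, icon and class, then destroys itself.
; ContextActivate and ContextDeactivate show and clear a context menu on its widget component, built from the item's button list.
; Drop is an empty stub.
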(event `self.ReceiveTick`
  (params (DeltaSeconds :type "Float (single-precision)"))
  (`parent.ReceiveTick` DeltaSeconds))

(event `/Game/Blueprints/UI/ContextMenu/IContextInteractible.ContextActivate`
  (params (NewParam :type Boolean))
  (bind _returnvalue (`|CreateWidget` "/Game/Blueprints/UI/ContextMenu/ContextMenu_Widget.ContextMenu_Widget_C" null (`self.ContextMenuButtons`) self))
  (`WidgetComponent.SetWidget` (`self.WidgetContext`) _returnvalue))

(event `/Game/Blueprints/UI/ContextMenu/IContextInteractible.ContextDeactivate`
  (`WidgetComponent.SetWidget` (`self.WidgetContext`) null))

(fn `Drop`
  (params (Inventory :type "/Game/Blueprints/Inventory/InventoryCOmponent Object Reference"))
  (returns (Item :type "/Game/Blueprints/Items/ItemBase Object Reference"))
  (return null))

(fn `EndInteraction`
  (params (Player :type "/Game/Blueprints/Player/Player_Pawn Object Reference"))
  (returns (ret :type Boolean))
  (`self.K2_DestroyActor`)
  (return false))

(fn `StartInteraction`
  (params (Player :type "/Game/Blueprints/Player/Player_Pawn Object Reference"))
  (returns (ret :type Boolean))
  (bind _returnvalue (`self.GetComponentByClass` Player "/Game/Blueprints/Inventory/InventoryCOmponent.InventoryComponent_C"))
  (`/Engine/EditorBlueprintResources/StandardMacros.IsValid` _returnvalue
    (:`Is Valid`
      (if (not (`/Game/Blueprints/Inventory/InventoryCOmponent.isFilled` _returnvalue))
        (bind _inventoryitem (`self.Stash` _returnvalue))
        (`/Game/Blueprints/Inventory/InventoryCOmponent.StashItem` _returnvalue _inventoryitem)
        (`self.SetActorHiddenInGame` true)
        (`self.EndInteraction` Player)))))

(fn `Stash`
  (params (Inventory :type "/Game/Blueprints/Inventory/InventoryCOmponent Object Reference"))
  (returns (InventoryItem :type "/Game/Blueprints/Inventory/InventoryItem Object Reference"))
  (bind _returnvalue (`|GenericCreateObject` "/Game/Blueprints/Inventory/InventoryItem.InventoryItem_C" Inventory (`self.Name`) (`self.Weight`) (`self.InventoryIcon`) (`GameplayStatics.GetObjectClass` self)))
  (`self.SetActorHiddenInGame` self true)
  (return _returnvalue))

(fn `UserConstructionScript`
  (`parent.UserConstructionScript`))