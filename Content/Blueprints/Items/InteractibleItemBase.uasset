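; Base Blueprint for interactable items, with handlers for highlight and interaction start and end.
; Highlight start and end both toggle custom depth rendering on the static mesh rather than setting it explicitly.
; Starting interaction stores the player as InteractivePawn and swaps the mesh material, while ending clears the pawn and applies a wall material.
; All four handlers return false, and the StartInt/EndInt gate leads only to an empty FlipFlop.
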(event `self.ReceiveTick`
  (params (DeltaSeconds :type "Float (single-precision)"))
  (`parent.ReceiveTick` DeltaSeconds))

(event `StartInt`
  (`/Engine/EditorBlueprintResources/StandardMacros.Gate` true :!via `Open` :!label _label
    (:`Exit`
      (`/Engine/EditorBlueprintResources/StandardMacros.FlipFlop`))))

(event `EndInt`
  (goto _label :!via `Close`))

(fn `EndInteraction`
  (params (Player :type "/Game/Blueprints/Player/Player_Pawn Object Reference"))
  (returns (ret :type Boolean))
  (set `self.InteractivePawn` null)
  (`PrimitiveComponent.SetMaterial` (`self.StaticMesh`) 0 "/Game/StarterContent/Materials/M_Basic_Wall.M_Basic_Wall")
  (return false))

(fn `OnEndHighlite`
  (params (Player :type "/Game/Blueprints/Player/Player_Pawn Object Reference"))
  (returns (ret :type Boolean))
  (`self.ToggleHighlite`)
  (return false))

(fn `OnStartHighlite`
  (params (Player :type "/Game/Blueprints/Player/Player_Pawn Object Reference"))
  (returns (ret :type Boolean))
  (`self.ToggleHighlite`)
  (return false))

(fn `StartInteraction`
  (params (Player :type "/Game/Blueprints/Player/Player_Pawn Object Reference"))
  (returns (ret :type Boolean))
  (set `self.InteractivePawn` Player)
  (`PrimitiveComponent.SetMaterial` (`self.StaticMesh`) 0 "/Game/StarterContent/Blueprints/Assets/M_LightStage_Skybox_HDRI.M_LightStage_Skybox_HDRI")
  (return false))

(fn `ToggleHighlite`
  (bind _staticmesh (`self.StaticMesh`))
  (`PrimitiveComponent.SetRenderCustomDepth` _staticmesh (not (`PrimitiveComponent.bRenderCustomDepth` _staticmesh))))

(fn `UserConstructionScript`
  (`parent.UserConstructionScript`))